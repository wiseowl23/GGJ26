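; BP_GuardSpawn is a spawner actor that, judging by its naming, places a group of guards in the level.
; Its SpawnGuards event spawns four actors in sequence at the world locations of its Loc1, StaticMesh, StaticMesh1 and StaticMesh2 components, which act as position markers.
; All spawns share one fixed rotation, and nothing in the Blueprint itself calls the event.
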(event Custom|SpawnGuards
  (Game|SpawnActorfromClass "/Game/Blueprints/Drones/BP_Office_Security.BP_Office_Security_C" (Math|Transform|MakeTransform (Transformation|GetWorldLocation (Variables|Default|GetLoc1)) "0.000000,-90.000000,0.000000" "1.000000,1.000000,1.000000") "Undefined" "MultiplyWithRoot" 0 0)
  (Game|SpawnActorfromClass "/Game/Blueprints/Drones/BP_Office_Security.BP_Office_Security_C" (Math|Transform|MakeTransform (Transformation|GetWorldLocation (Variables|Default|GetStaticMesh)) "0.000000,-90.000000,0.000000" "1.000000,1.000000,1.000000") "Undefined" "MultiplyWithRoot" 0 0)
  (Game|SpawnActorfromClass "/Game/Blueprints/Drones/BP_Office_Security.BP_Office_Security_C" (Math|Transform|MakeTransform (Transformation|GetWorldLocation (Variables|Default|GetStaticMesh1)) "0.000000,-90.000000,0.000000" "1.000000,1.000000,1.000000") "Undefined" "MultiplyWithRoot" 0 0)
  (Game|SpawnActorfromClass "/Game/Blueprints/Drones/BP_Office_Security.BP_Office_Security_C" (Math|Transform|MakeTransform (Transformation|GetWorldLocation (Variables|Default|GetStaticMesh2)) "0.000000,-90.000000,0.000000" "1.000000,1.000000,1.000000") "Undefined" "MultiplyWithRoot" 0 0))

(fn ConstructionScript)