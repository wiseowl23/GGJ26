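; BP_HRDoor is an interactable HR door that acts only while the player character's MissionStage is 5.
; Its Interact event looks up the HR_SpawnPoint actor, leaves the result unused, and calls SitDown on BP_PlayerCharacter.
; Beginning an overlap with InteractRadius at that stage hides the Widget component.
; End overlap and the construction script are empty.
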(event OnComponentBeginOverlap(InteractRadius)
  (params (OverlappedComponent :type Primitive%20Component%20Object%20Reference) (OtherActor :type Actor%20Object%20Reference) (OtherComp :type Primitive%20Component%20Object%20Reference) (OtherBodyIndex :type Integer) (bFromSweep :type Boolean) (SweepResult :type Hit%20Result%20Structure%20%28by%20ref%29))
  (bind _asbp_player_character (Utilities|Casting|CastToBP_PlayerCharacter (Game|GetPlayerCharacter 0)))
  (if (== (Variables|/Game/Blueprints/Player/BP_PlayerCharacter.BP_PlayerCharacter_C|GetMissionStage _asbp_player_character) 5)
    (Rendering|SetVisibility (Variables|Default|GetWidget) false false)))

(event OnComponentEndOverlap(InteractRadius)
  (params (OverlappedComponent :type Primitive%20Component%20Object%20Reference) (OtherActor :type Actor%20Object%20Reference) (OtherComp :type Primitive%20Component%20Object%20Reference) (OtherBodyIndex :type Integer)))

(event EventInteract
  (bind _asbp_player_character (Utilities|Casting|CastToBP_PlayerCharacter (Game|GetPlayerCharacter 0)))
  (if (== (Variables|/Game/Blueprints/Player/BP_PlayerCharacter.BP_PlayerCharacter_C|GetMissionStage _asbp_player_character) 5)
    (Actor|GetActorOfClass "/Game/Blueprints/HR_SpawnPoint.HR_SpawnPoint_C")
    (Default|SitDown _asbp_player_character)))

(fn ConstructionScript)