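; Dialogue component that opens and closes the dialogue UI and relays dialogue trigger events.
; StartDialogue creates WBP_Dialogue_Main from a first row name and itself, then switches to UI-only input with the mouse cursor shown.
; A DoOnce blocks repeat starts until EndDialogue removes the widget, restores game input and resets it.
; DialogueTrigger broadcasts OnDialogueEventTriggered for any trigger name other than None.
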(event Custom|StartDialogue
  (params (FirstRowName :type Name))
  (bind _returnvalue (Game|GetPlayerController 0))
  ;[0.06404 0.15 0.08461 0.5] Start dialogue
  (Utilities|FlowControl|DoOnce false
    (:Completed
      (bind _returnvalue_2 (UserInterface|CreateWidget "/Game/Blueprints/Dialogue/WBP_Dialogue_Main.WBP_Dialogue_Main_C" 0 FirstRowName self))
      (bind _output_get (Variables|Default|SetDialogue_Widget _returnvalue_2))
      (UserInterface|Viewport|AddtoViewport _output_get 0)
      (Input|SetInputModeUIOnly _returnvalue _output_get "DoNotLock" false)
      (Variables|/Script/Engine.PlayerController|SetbShowMouseCursor _returnvalue true))))

(event Custom|EndDialogue
  (bind _returnvalue (Game|GetPlayerController 0))
  (bind _returnvalue_2 (Game|GetPlayerController 0))
  ;[0.01385 0.0595 0.15 0.5] End dialogue
  (Widget|RemovefromParent (Variables|Default|GetDialogue_Widget))
  (Variables|/Script/Engine.PlayerController|SetbShowMouseCursor _returnvalue_2 false)
  (Input|SetInputModeGameOnly _returnvalue_2 false)
  (Variables|Default|SetDialogue_Widget 0)
  ;[0.06404 0.15 0.08461 0.5] Start dialogue
  (Utilities|FlowControl|DoOnce false) ; enters at Reset
)

(event Custom|DialogueTrigger
  (params (TriggerName :type Name))
  (if (!= TriggerName "")
    (Default|CallOnDialogueEventTriggered TriggerName)))